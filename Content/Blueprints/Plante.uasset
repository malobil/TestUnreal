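; Plant actor that counts down a growing time and can be removed by interaction once grown.
; A looping one-second timer decrements the remaining time, shows it on the STATE text component, and clears itself at zero.
; Tick turns that text to face the player pawn.
; Interact calls the parent implementation, then destroys the actor if growth has finished.
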(event `self.ReceiveBeginPlay`
  (`self.Initialize`)
  (`KismetSystemLibrary.K2_SetTimer` null "DecreaseGrowingTime" 1.0 true))

(event `self.ReceiveTick`
  (params (DeltaSeconds :type "Float (single-precision)"))
  (bind _state (`self.STATE`))
  (`SceneComponent.K2_SetWorldRotation` _state (`KismetMathLibrary.Conv_VectorToRotator` (`KismetMathLibrary.Conv_RotatorToVector` (`KismetMathLibrary.FindLookAtRotation` (`SceneComponent.K2_GetComponentLocation` _state) (`self.K2_GetActorLocation` (`GameplayStatics.GetPlayerPawn` 0))))) false false))

(fn `DecreaseGrowingTime`
  (bind _output_get (set `self.CurrentGrowingTime` (- (`self.CurrentGrowingTime`) 1)))
  (`self.UpdateGrowingTimeText` (`KismetStringLibrary.Conv_IntToString` _output_get)))

(fn `Initialize`
  (bind _output_get (set `self.CurrentGrowingTime` (`self.GrowingTime`)))
  (`self.UpdateGrowingTimeText` (`KismetStringLibrary.Conv_IntToString` _output_get)))

(fn `Interact`
  (`parent.Interact`)
  (if (<= (`self.CurrentGrowingTime`) 0)
    (`self.K2_DestroyActor`)))

(fn `UpdateGrowingTimeText`
  (params (TextToShow :type String))
  (`TextRenderComponent.K2_SetText` (`self.STATE`) (`KismetTextLibrary.Conv_StringToText` TextToShow))
  (if (<= (`self.CurrentGrowingTime`) 0)
    (`KismetSystemLibrary.K2_ClearTimer` null "DecreaseGrowingTime")))

(fn `UserConstructionScript`)