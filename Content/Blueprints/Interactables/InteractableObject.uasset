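; Interactable actor whose response to interaction is built from attached InteractableBehavior components.
; On BeginPlay it orders those components by ascending Priority, using a selection sort that repeatedly takes the minimum and overwrites it with a large sentinel.
; Each sorted component's name is printed.
; Interact checks CanInteract, then calls TriggerBehavior on each behavior in that order, without passing on the Interactor.
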(event `self.ReceiveBeginPlay`
  (`self.Initialize`))

(fn `Initialize`
  (`self.Sort Component by Priority`))

(fn `Interact`
  (params (Interactor :type "Actor Object Reference"))
  (if (`self.CanInteract`)
    (for _array_element (`self.InteractableBehaviors`)
      (`/Game/Blueprints/Interactables/Behaviors/InteractableBehavior.TriggerBehavior` _array_element))))

(fn `Sort Component by Priority`
  (bind _tempinteractablebehaviors (`self.TempInteractableBehaviors`))
  (bind _indexofminvalue (`KismetMathLibrary.MinOfIntArray` (`self.TempPriorityStorage`)))
  ;[1 1 1] SortComponentByPriority
  (bind _output_get (set `self.TempInteractableBehaviors` (`self.K2_GetComponentsByClass` "/Game/Blueprints/Interactables/Behaviors/InteractableBehavior.InteractableBehavior_C")))
  (for _index (range (`KismetArrayLibrary.Array_Length` _output_get))
    (`KismetArrayLibrary.Array_Add` (`self.TempPriorityStorage`) (`/Game/Blueprints/Interactables/Behaviors/InteractableBehavior.Priority` (`|GetArrayItem` _tempinteractablebehaviors _index))))
  (for _ (range (`KismetArrayLibrary.Array_Length` _tempinteractablebehaviors))
    (bind _returnvalue (`KismetArrayLibrary.Array_Add` (`self.InteractableBehaviors`) (`|GetArrayItem` (`self.TempInteractableBehaviors`) _indexofminvalue)))
    (`KismetArrayLibrary.Array_Set` (`self.TempPriorityStorage`) _indexofminvalue 99999999)
    (`KismetSystemLibrary.PrintString` (`KismetSystemLibrary.GetDisplayName` (`|GetArrayItem` (`self.InteractableBehaviors`) _returnvalue)))))

(fn `UserConstructionScript`)